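; BP_InteractableItemBase is a base Blueprint for interactable items that shows an interaction prompt while a player is in range.
; On range entry, it creates a WBP_Interact widget for that player's controller and attaches it through a dynamically added, screen-space, collision-free WidgetComponent.
; GetInteractionText and GetInteractionTextAttach supply the label and attach point, defaulting to "Interact" and the root component.
; On range exit, it destroys the widget component.
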(event `/Game/Core/Interfaces/BPI_Interact.OnInteractionRangeEntered`
  (params (Player :type "/Game/Core/FirstPerson/Blueprints/BP_FirstPersonCharacter Object Reference"))
  (`self.InteractionWidgetCompnent`
    (:`then`)
    (:`else`
      (bind _returnvalue (`|CreateWidget` "/Game/UI/WBP_Interact.WBP_Interact_C" (cast `PlayerController` (`Pawn.GetController` Player) :!pure true) (`self.GetInteractionText`)))
      (bind _returnvalue_2 (`AddComponent|NODE_AddWidgetComponent-0`))
      (bind _output_get (set `self.InteractionWidgetCompnent` _returnvalue_2))
      (`WidgetComponent.SetWidget` _output_get _returnvalue)
      (`WidgetComponent.SetWidgetSpace` _output_get "Screen")
      (`WidgetComponent.SetDrawAtDesiredSize` _output_get true)
      (`PrimitiveComponent.SetCollisionEnabled` _output_get "NoCollision")
      (`SceneComponent.K2_AttachToComponent` _output_get (`self.GetInteractionTextAttach`) "None" "SnapToTarget" "SnapToTarget" "SnapToTarget" true))))

(event `/Game/Core/Interfaces/BPI_Interact.OnInteractionRangeExited`
  (bind _interactionwidgetcompnent (`self.InteractionWidgetCompnent`)
    (:`then`
      (`ActorComponent.K2_DestroyComponent` _interactionwidgetcompnent))
    (:`else`)))

(fn `GetInteractionText`
  (returns (Text :type Text))
  (return "Interact"))

(fn `GetInteractionTextAttach`
  (returns (AttachComponent :type "SceneComponent Object Reference"))
  (return (`self.DefaultSceneRoot`)))

(fn `UserConstructionScript`)