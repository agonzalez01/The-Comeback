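; Health and armor component that tracks both values on its owning actor and reacts to the damage it takes.
; On BeginPlay it binds to the owner's any-damage event and optionally fills health and armor to their maximums.
; Armor absorbs damage first, with the overflow reducing health, and clamped setters broadcast change events.
; After each hit it fires a death event at zero health, otherwise a damage event.
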(event `self.ReceiveBeginPlay`
  (add `Actor.OnTakeAnyDamage` (`self.GetOwner`) (delegate `ProcessDamage`))
  (if (`self.MaxOnStart`)
    (`self.SetCurrentHealth` (`self.MaxHealth`))
    (`self.SetCurrentArmor` (`self.MaxArmor`))))

(event `ProcessDamage`
  (params (DamagedActor :type "Actor Object Reference") (Damage :type "Float (single-precision)") (DamageType :type "DamageType Object Reference") (InstigatedBy :type "Controller Object Reference") (DamageCauser :type "Actor Object Reference"))
  (`self.UpdateHealthArmor` Damage))

(fn `GetArmorRatio`
  (returns (Ration :type "Float (double-precision)"))
  (return (/ (`self.CurrentArmor`) (`self.MaxArmor`))))

(fn `GetCurrentArmor`
  (returns (CurrentArmor :type "Float (double-precision)"))
  (return (`self.CurrentArmor`)))

(fn `GetCurrentHealth`
  (returns (CurrentHealth :type "Float (double-precision)"))
  (return (`self.CurrentHealth`)))

(fn `GetHealthRatio`
  (returns (Ratio :type "Float (double-precision)"))
  (return (/ (`self.CurrentHealth`) (`self.MaxHealth`))))

(fn `SetCurrentArmor`
  (params (Value :type "Float (double-precision)"))
  (set `self.CurrentArmor` (`KismetMathLibrary.FClamp` Value 0.0 (`self.MaxArmor`)))
  (`self.OnArmorChanged`))

(fn `SetCurrentHealth`
  (params (Value :type "Float (double-precision)"))
  (set `self.CurrentHealth` (`KismetMathLibrary.FClamp` Value 0.0 (`self.MaxHealth`)))
  (`self.OnHealthChanged`))

(fn `UpdateHealthArmor`
  (params (Damage :type "Float (double-precision)"))
  (locals (ArmorDamage :type "Float (double-precision)") (HealthDamage :type "Float (double-precision)"))
  (set `local.ArmorDamage` (`KismetMathLibrary.FMin` Damage (`self.CurrentArmor`)))
  (set `local.HealthDamage` (`KismetMathLibrary.FClamp` (- Damage (`self.CurrentArmor`)) 0.0 (`self.MaxHealth`)))
  (`self.SetCurrentArmor` (`KismetMathLibrary.FClamp` (- (`self.CurrentArmor`) (`local.ArmorDamage`)) 0.0 (`self.MaxArmor`)))
  (`self.SetCurrentHealth` (`KismetMathLibrary.FClamp` (- (`self.CurrentHealth`) (`local.HealthDamage`)) 0.0 (`self.MaxHealth`)))
  (if (<= (`self.GetHealthRatio`) 0.0)
    (`self.OnDeath`)
    (else
      (`self.OnDamage`))))